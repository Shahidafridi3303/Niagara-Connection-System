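; Platform Blueprint that drives a weight mechanism through a referenced actor when the player character enters or leaves its Box1 trigger.
; Entering calls Start on BPWeightRef with a positive value, and leaving calls it with the matching negative value.
; Each event has its own FlipFlop, so successive entries, and likewise successive exits, alternate between that actor's Platform1 and Platform2 as the target.
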(event OnComponentBeginOverlap(Box1)
  (params (OverlappedComponent :type Primitive%20Component%20Object%20Reference) (OtherActor :type Actor%20Object%20Reference) (OtherComp :type Primitive%20Component%20Object%20Reference) (OtherBodyIndex :type Integer) (bFromSweep :type Boolean) (SweepResult :type Hit%20Result%20Structure%20%28by%20ref%29))
  (bind _bp_weight_ref (Variables|Default|GetBP_Weight%20Ref))
  (bind _bp_weight_ref_2 (Variables|Default|GetBP_Weight%20Ref))
  (Utilities|Casting|CastToBP_MyCharacter OtherActor)
  (Utilities|FlowControl|FlipFlop
    (:A
      (Default|Start _bp_weight_ref (Variables|/Game/Blueprints/BP_Weight.BP_Weight_C|GetPlatform1 _bp_weight_ref) 2.5))
    (:B
      (Default|Start _bp_weight_ref_2 (Variables|/Game/Blueprints/BP_Weight.BP_Weight_C|GetPlatform2 _bp_weight_ref_2) 2.5))))

(event OnComponentEndOverlap(Box1)
  (params (OverlappedComponent :type Primitive%20Component%20Object%20Reference) (OtherActor :type Actor%20Object%20Reference) (OtherComp :type Primitive%20Component%20Object%20Reference) (OtherBodyIndex :type Integer))
  (bind _bp_weight_ref (Variables|Default|GetBP_Weight%20Ref))
  (bind _bp_weight_ref_2 (Variables|Default|GetBP_Weight%20Ref))
  (Utilities|Casting|CastToBP_MyCharacter OtherActor)
  (Utilities|FlowControl|FlipFlop
    (:A
      (Default|Start _bp_weight_ref (Variables|/Game/Blueprints/BP_Weight.BP_Weight_C|GetPlatform1 _bp_weight_ref) -2.5))
    (:B
      (Default|Start _bp_weight_ref_2 (Variables|/Game/Blueprints/BP_Weight.BP_Weight_C|GetPlatform2 _bp_weight_ref_2) -2.5))))

(fn ConstructionScript)